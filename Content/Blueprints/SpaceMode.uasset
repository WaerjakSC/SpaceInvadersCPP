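; SpaceMode is a Blueprint that pauses the game once all enemies are gone, provided the player's ammo is also low.
; Each Tick, it reads the enemy count from the C++ SpaceCPP_GameModeBase.
; When that count is zero, it checks Ammo on the player's BP_CharPawn and pauses only if it is below a hardcoded threshold.
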(event EventTick
  (params (DeltaSeconds :type Float%20%28single-precision%29))
  ;[1 1 1] Pause if no enemies left
  (bind _asspace_cpp_game_mode_base (Utilities|Casting|CastToSpaceCPP_GameModeBase (Game|GetGameMode)))
  (if (== (Variables|/Script/SpaceCPP.SpaceCPP_GameModeBase|GetNumEnemies _asspace_cpp_game_mode_base) 0)
    (bind _asbp_char_pawn (Utilities|Casting|CastToBP_CharPawn (Game|Player|GetPlayerPawn 0)))
    (if (< (Variables|/Script/SpaceCPP.CharPawn|GetAmmo _asbp_char_pawn) 30)
      (Game|SetGamePaused true))))

(fn ConstructionScript)